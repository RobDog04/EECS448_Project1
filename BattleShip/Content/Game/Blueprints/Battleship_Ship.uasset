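; Draggable Battleship ship that players position and rotate on BattleshipBlock cells using mouse, touch or controller handlers.
; The construction script picks mesh, transform and capsule dimensions from ShipSize.
; Grabbing clears HasBoat on overlapped blocks and opens a Tick gate that follows the cursor trace in XY.
; Release marks blocks occupied if the overlap count equals ShipSize and all are free, otherwise restores the pre-grab transform.
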(event `self.ReceiveTick`
  (params (DeltaSeconds :type "Float (single-precision)"))
  (bind (_returnvalue_x _returnvalue_y _returnvalue_z) (`KismetMathLibrary.BreakVector` (`self.K2_GetActorLocation`)))
  (bind (_bblockinghit _binitialoverlap _time _distance _location) (`GameplayStatics.BreakHitResult` (`PlayerController.GetHitResultUnderCursorByChannel` (`GameplayStatics.GetPlayerController` 0) "TraceTypeQuery1" true)))
  (`/Engine/EditorBlueprintResources/StandardMacros.Gate` true :!label _label
    (:`Exit`
      (if (`self.CanGrab`)
        (`self.K2_SetActorLocation` (`KismetMathLibrary.MakeVector` (.x _location) (.y _location) _returnvalue_z))))))

(event `self.Capsule.OnClicked`
  (params (TouchedComponent :type "PrimitiveComponent Object Reference") (ButtonPressed :type "Key Structure"))
  (if (`self.CanGrab`)
    (if (not (`self.Grabbed`))
      (set `PlayerController.CurrentMouseCursor` "GrabHandClosed" (`GameplayStatics.GetPlayerController` 0))
      (set `self.Grabbed` true :!label _label_2)
      (bind _output_get (set `self.OriginTransform` (`self.GetTransform`)))
      (for _array_element (`PrimitiveComponent.GetOverlappingActors` (`self.Capsule`) "/Game/Game/Blueprints/BattleshipBlock.BattleshipBlock_C")
        (bind _asbattleship_block (cast `/Game/Game/Blueprints/BattleshipBlock` _array_element))
        (set `/Game/Game/Blueprints/BattleshipBlock.HasBoat` false _asbattleship_block))
      (goto _label :!via `Open`))))

(event `self.Capsule.OnInputTouchBegin`
  (params (FingerIndex :type "ETouchIndex Enum" :default "Touch1") (TouchedComponent :type "PrimitiveComponent Object Reference"))
  (bind (_returnvalue_roll _returnvalue_pitch _returnvalue_yaw) (`KismetMathLibrary.BreakRotator` (`self.K2_GetActorRotation`)))
  (if (`self.CanGrab`)
    (if (== FingerIndex 1)
      (if (not (`self.Grabbed`)) :!label _label_3
        (goto _label_2))
      (else
        ;[1 1 1] TODO: Fix second finger touch rotation
        (`KismetSystemLibrary.PrintString` "Second Touch detected")
        (if (`self.Grabbed`) :!label _label_4
          (`self.K2_SetActorRotation` (`KismetMathLibrary.MakeRotator` 0.0 0.0 (+ _returnvalue_yaw 90.0))))))))

(event `HandleControllerClick`
  (if (`self.CanGrab`)
    (goto _label_3)))

(event `self.Capsule.OnReleased`
  (params (TouchedComponent :type "PrimitiveComponent Object Reference") (ButtonReleased :type "Key Structure"))
  (bind _overlappingactors (`PrimitiveComponent.GetOverlappingActors` (`self.Capsule`) "/Game/Game/Blueprints/BattleshipBlock.BattleshipBlock_C"))
  (if (`self.CanGrab`)
    (if (`self.Grabbed`)
      (set `PlayerController.CurrentMouseCursor` "GrabHand" (`GameplayStatics.GetPlayerController` 0))
      (set `self.Grabbed` false :!label _label_5)
      (if (`self.IsValidDropLocation`)
        (for _array_element _overlappingactors
          (bind _asbattleship_block (cast `/Game/Game/Blueprints/BattleshipBlock` _array_element))
          (`/Game/Game/Blueprints/BattleshipBlock.UnHighlight` _asbattleship_block)
          (if (`/Game/Game/Blueprints/BattleshipBlock.HasBoat` _asbattleship_block)
            (set `self.IsValidDropLocation` false)))
        (if (`self.IsValidDropLocation`)
          (for _array_element_2 _overlappingactors
            (bind _asbattleship_block_2 (cast `/Game/Game/Blueprints/BattleshipBlock` _array_element_2))
            (set `/Game/Game/Blueprints/BattleshipBlock.HasBoat` true _asbattleship_block_2))
          (goto _label :!via `Close`)
          (else
            _)))
      (`self.K2_SetActorTransform` (stale `self.Capsule.OnClicked` _output_get))
      (goto _label :!via `Close`))))

(event `self.Capsule.OnInputTouchEnd`
  (params (FingerIndex :type "ETouchIndex Enum" :default "Touch1") (TouchedComponent :type "PrimitiveComponent Object Reference"))
  (if (`self.CanGrab`)
    (if (== FingerIndex 1)
      (if (`self.Grabbed`) :!label _label_6
        (goto _label_5)))))

(event `InputAction|OnRightClick` :consume false :overrideparent false
  (params (Key :type "Key Structure"))
  ;[1 1 1] TODO: Fix second finger touch rotation
  (:`Pressed`
    (goto _label_4)))

(event `HandleControllerEndClick`
  (if (`self.CanGrab`)
    (goto _label_6)))

(event `Key|SpaceBar` :consume false :overrideparent false
  (params (Key :type "Key Structure"))
  ;[1 1 1] TODO: Fix second finger touch rotation
  (:`Pressed`
    (goto _label_4)))

(event `self.Capsule.OnComponentBeginOverlap`
  (params (OverlappedComponent :type "PrimitiveComponent Object Reference") (OtherActor :type "Actor Object Reference") (OtherComp :type "PrimitiveComponent Object Reference") (OtherBodyIndex :type Integer) (bFromSweep :type Boolean) (SweepResult :type "HitResult Structure (by ref)"))
  (if (== (`GameplayStatics.GetObjectClass` OtherActor) "/Game/Game/Blueprints/BattleshipBlock.BattleshipBlock_C")
    (set `self.OverlappingBlocks` (+ (`self.OverlappingBlocks`) 1))
    (if (== (`self.OverlappingBlocks`) (`self.ShipSize`))
      (set `self.IsValidDropLocation` true :!label _label_7)
      (else
        (set `self.IsValidDropLocation` false :!label _label_8)))))

(event `self.Capsule.OnBeginCursorOver`
  (params (TouchedComponent :type "PrimitiveComponent Object Reference"))
  (if (`self.CanGrab`)
    (set `PlayerController.CurrentMouseCursor` "GrabHand" (`GameplayStatics.GetPlayerController` 0))))

(event `self.Capsule.OnEndCursorOver`
  (params (TouchedComponent :type "PrimitiveComponent Object Reference"))
  (set `PlayerController.CurrentMouseCursor` "Default" (`GameplayStatics.GetPlayerController` 0)))

(event `self.Capsule.OnComponentEndOverlap`
  (params (OverlappedComponent :type "PrimitiveComponent Object Reference") (OtherActor :type "Actor Object Reference") (OtherComp :type "PrimitiveComponent Object Reference") (OtherBodyIndex :type Integer))
  (if (== (`GameplayStatics.GetObjectClass` OtherActor) "/Game/Game/Blueprints/BattleshipBlock.BattleshipBlock_C")
    (set `self.OverlappingBlocks` (- (`self.OverlappingBlocks`) 1))
    (if (== (`self.OverlappingBlocks`) (`self.ShipSize`))
      (goto _label_7)
      (else
        (goto _label_8)))))

(fn `UserConstructionScript`
  (bind _shipsize (`self.ShipSize`))
  (bind _capsule (`self.Capsule`))
  (bind _capsule_2 (`self.Capsule`))
  (bind _capsule_3 (`self.Capsule`))
  (bind _capsule_4 (`self.Capsule`))
  (bind _capsule_5 (`self.Capsule`))
  (bind _capsule_6 (`self.Capsule`))
  (bind _ship (`self.Ship`))
  (bind _ship_2 (`self.Ship`))
  (switch `int` (`self.ShipSize`)
    (:`1`
      (`StaticMeshComponent.SetStaticMesh` _ship_2 "/Game/Game/Meshes/Rowboat.Rowboat" :!label _label)
      (switch `int` _shipsize
        (:`1`
          (`SceneComponent.K2_SetRelativeTransform` _ship (`self.1x1_Transform`) false false)
          (`CapsuleComponent.SetCapsuleHalfHeight` _capsule_2 110.0 true)
          (`CapsuleComponent.SetCapsuleRadius` _capsule_2 45.0 true))
        (:`2`
          (`SceneComponent.K2_SetRelativeTransform` _ship (`self.1x2_Transform`) false false)
          (`CapsuleComponent.SetCapsuleHalfHeight` _capsule_3 220.0 true)
          (`CapsuleComponent.SetCapsuleRadius` _capsule_3 100.0 true))
        (:`3`
          (`SceneComponent.K2_SetRelativeTransform` _ship (`self.1x3_Transform`) false false)
          (`CapsuleComponent.SetCapsuleHalfHeight` _capsule_4 340.0 true)
          (`CapsuleComponent.SetCapsuleRadius` _capsule_4 100.0 true))))
    (:`2`
      (goto _label))
    (:`3`
      (goto _label))
    (:`4`
      (`StaticMeshComponent.SetStaticMesh` _ship_2 "/Game/Game/Meshes/SailingShip.SailingShip" :!label _label_2)
      (switch `int` _shipsize
        (:`4`
          (`SceneComponent.K2_SetRelativeTransform` _ship (`self.1x4_Transform`) false false)
          (`CapsuleComponent.SetCapsuleHalfHeight` _capsule_5 480.0 true)
          (`CapsuleComponent.SetCapsuleRadius` _capsule_5 100.0 true))
        (:`5`
          (`SceneComponent.K2_SetRelativeTransform` _ship (`self.1x5_Transform`) false false)
          (`CapsuleComponent.SetCapsuleHalfHeight` _capsule_6 600.0 true)
          (`CapsuleComponent.SetCapsuleRadius` _capsule_6 100.0 true))
        (:`6`
          (`SceneComponent.K2_SetRelativeTransform` _ship (`self.1x6_Transform`) false false)
          (`CapsuleComponent.SetCapsuleHalfHeight` _capsule 720.0 true)
          (`CapsuleComponent.SetCapsuleRadius` _capsule 100.0 true))))
    (:`5`
      (goto _label_2))
    (:`6`
      (goto _label_2)))
  (set `self.OriginTransform` (`self.GetTransform`)))