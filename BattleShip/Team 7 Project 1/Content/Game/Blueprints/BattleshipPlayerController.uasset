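; Player controller for Battleship that handles game mode setup, menu and status widgets, and match flow for single-player and two-player LAN games.
; Session events host or join LAN games, and GameInstance carries role and ship count across level loads.
; Host/client branches write connection, ready, turn and attack state to GameState, whose bound notifications drive turn changes, sunk-ship and win/lose feedback.
; A delayed retry waits for a valid GameState on BeginPlay.
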(event `SetupSinglePlayerMode`
  ;[1 1 1] Sets up single player mode
  (set `/Game/Game/Blueprints/BattleshipGameInstance.ShipCount` (`/Game/Game/Blueprints/BattleShipGameState.ShipCount` (`self.GameState`)) (`self.GameInstance`))
  (`GameplayStatics.OpenLevel` "Battleship_MainGameMap"))

(event `SetupHostMode`
  ;[1 1 1] Setup Server Host Connection and Reopen Level in ?listen for Client connection state
  (`CreateSessionCallbackProxy.CreateSession` self 2 true
    (:`OnSuccess`
      (set `/Game/Game/Blueprints/BattleshipGameInstance.ShipCount` (`/Game/Game/Blueprints/BattleShipGameState.ShipCount` (`self.GameState`)) (`self.GameInstance`))
      (`GameplayStatics.OpenLevel` "Battleship_MainGameMap" true "?listen") ; Restarts the level and listens for player connection
    )))

(event `self.ReceiveBeginPlay`
  (bind (_asbattle_ship_game_state _bsuccess) (cast `/Game/Game/Blueprints/BattleShipGameState` (`GameplayStatics.GetGameState`) :!pure true))
  ;[1 1 1] Determine if the Player Has Selected a Game Mode (GameInstance)
  (bind _returnvalue (`GameplayStatics.GetCurrentLevelName` true))
  (if (`KismetStringLibrary.EqualEqual_StrStr` _returnvalue "Battleship_MainGameMap")
    (if _bsuccess :!label _label
      (set `self.GameState` _asbattle_ship_game_state)
      (set `self.GameInstance` (cast `/Game/Game/Blueprints/BattleshipGameInstance` (`GameplayStatics.GetGameInstance`) :!pure true))
      (`self.IsPlayer#`
        (:`1 (Host)`
          ;[1 1 1] If Host Mode Selected Notify GameState of Player 1 Connected
          (`self.SetGameStateShipCount`)
          (`self.AskLevelToUpdateShips`)
          (`self.UpdatePlayer1ConnectedInGameState` true)
          (`self.SetupPlayer1Bindings`)
          (`self.DisplayWaitingForPlayerToConnect`))
        (:`2 (Client)`
          ;[1 1 1] If Join Mode Selected Notify GameState of Player 2 Connected
          (`self.DisplayConnectingToGameHost`)
          (`self.AskLevelToUpdateShips`)
          (`self.UpdatePlayer2ConnectedInGameState` true)
          (`self.SetupPlayer2Bindings`))
        (:`Neither`
          ;[1 1 1] If Game Mode Not Selected Yet
          (`self.DisplayHostOrJoin`)))
      (else
        (`KismetSystemLibrary.Delay` 0.2)
        (goto _label)))))

(event `SetupClientMode`
  ;[1 1 1] Connect to a Hosted LAN Server as a Client. Also display a "Connecting to Host" UI until connection established
  (bind _results (`FindSessionsCallbackProxy.FindSessions` self 2 true)
    (:`then`
      (`self.DisplayConnectingToGameHost`))
    (:`OnSuccess`
      (`JoinSessionCallbackProxy.JoinSession` self (`|GetArrayItem` _results)))))

(event `PassShipsToAI`
  (params (PlayerShipLocations :type "Array of /Game/Game/Blueprints/AI_Block_Struct Structure"))
  ;[1 1 1] Returns ship locations
  (`/Game/Game/Blueprints/BattleShipGameState.HandleShipsForAI` (`self.GameState`) PlayerShipLocations))

(event `UpdatePlayer1ConnectedInGameState`
  (params (SetPlayer1Connected :type Boolean))
  ;[1 1 1] Update Server (GameState) with Player 1 Connected (Run on Server Only)
  (set `/Game/Game/Blueprints/BattleShipGameState.Player1Connected` SetPlayer1Connected (`self.GameState`)))

(event `UpdatePlayer2ConnectedInGameState`
  (params (SetPlayer2Connected :type Boolean))
  ;[1 1 1] Update Server (GameState) with Player 2 Connected (Run on Server Only)
  (set `/Game/Game/Blueprints/BattleShipGameState.Player2Connected` SetPlayer2Connected (`self.GameState`)))

(event `DisplayWinLose`
  (params (Player1Win :type Boolean) (Player2Win :type Boolean))
  ;[1 1 1] Handle Win/Lose Conditions
  (`self.IsPlayer#`
    (:`1 (Host)`
      (if Player1Win
        (`GameplayStatics.PlaySound2D` "/Game/StarterContent/Audio/Taps_Cue.Taps_Cue" 1.0 1.0 0.0 null null :!label _label_2)
        (`self.DisplayWin`)
        (else
          (`GameplayStatics.PlaySound2D` "/Game/StarterContent/Audio/Taps_Cue.Taps_Cue" 1.0 1.0 0.0 null null :!label _label_3)
          (`self.DisplayLose`))))
    (:`2 (Client)`
      (if Player2Win
        (goto _label_2)
        (else
          (goto _label_3))))))

(event `UpdatePlayer1ReadyInGameState`
  (params (SetPlayer1Ready :type Boolean))
  ;[1 1 1] Update Server (GameState) with Player 1 Ready (Run on Server Only)
  (set `/Game/Game/Blueprints/BattleShipGameState.Player1Ready` SetPlayer1Ready (`self.GameState`)))

(event `UpdatePlayer2ReadyInGameState`
  (params (SetPlayer2Ready :type Boolean))
  ;[1 1 1] Update Server (GameState) with Player 2 Ready (Run on Server Only)
  (set `/Game/Game/Blueprints/BattleShipGameState.Player2Ready` SetPlayer2Ready (`self.GameState`)))

(event `SetGameStateShipCount`
  ;[1 1 1] Set (GameState) Ship Count using Game Instance
  (set `/Game/Game/Blueprints/BattleShipGameState.ShipCount` (`/Game/Game/Blueprints/BattleshipGameInstance.ShipCount` (`self.GameInstance`)) (`self.GameState`)))

(event `InitiateGamePlay`
  (bind _gamestate (`self.GameState`))
  ;[1 1 1] Initiate Random Start Player
  (set `/Game/Game/Blueprints/BattleShipGameState.StartRole` (`KismetMathLibrary.RandomBool`) _gamestate)
  (`KismetSystemLibrary.Delay` 1.0)
  (set `/Game/Game/Blueprints/BattleShipGameState.InitiateGamePlay` true _gamestate))

(event `UpdatePlayer1TurnInGameState`
  (params (SetPlayer1Turn :type Boolean))
  ;[1 1 1] Update Server (GameState) with Player 1 Turn Status (Run on Server Only)
  (set `/Game/Game/Blueprints/BattleShipGameState.Player1Turn` SetPlayer1Turn (`self.GameState`)))

(event `UpdatePlayer2TurnInGameState`
  (params (SetPlayer2Turn :type Boolean))
  ;[1 1 1] Update Server (GameState) with Player 2 Turn Status (Run on Server Only)
  (set `/Game/Game/Blueprints/BattleShipGameState.Player2Turn` SetPlayer2Turn (`self.GameState`)))

(event `AnnounceReadyToPlay`
  (bind _gamestate (`self.GameState`))
  ;[1 1 1] Announce to (GameState) Ready to play
  (`self.IsPlayer#`
    (:`1 (Host)`
      (`self.SetupPlayer1BindingsPart2`)
      (`self.UpdatePlayer1ReadyInGameState` true)
      (if (`/Game/Game/Blueprints/BattleShipGameState.Player2Ready` _gamestate)
        (`self.InitiateGamePlay` :!label _label_4)
        (else
          (`self.DisplayWaitingForPlayerToPlaceShips` :!label _label_5))))
    (:`2 (Client)`
      (`self.SetupPlayer2BindingsPart2`)
      (`self.UpdatePlayer2ReadyInGameState` true)
      (if (`/Game/Game/Blueprints/BattleShipGameState.Player1Ready` _gamestate)
        (goto _label_4)
        (else
          (goto _label_5))))))

(event `AttackBlock`
  (params (GameBoardPosition :type Integer))
  ;[1 1 1] Update Server (GameState) with Block Currently under attack
  (set `/Game/Game/Blueprints/BattleShipGameState.AttackedBlock` GameBoardPosition (`self.GameState`)))

(event `SendShipHit`
  (params (SetShipHit :type Boolean))
  ;[1 1 1] Update Server (GameState) with Ship Hit (Run on Server Only)
  (set `/Game/Game/Blueprints/BattleShipGameState.ShipHit` SetShipHit (`self.GameState`)))

(event `ResetShipSunk`
  ;[1 1 1] Resets ships
  (set `/Game/Game/Blueprints/BattleShipGameState.ShipSunk` false (`self.GameState`)))

(event `HandleChangeTurns`
  (params (Player1Turn :type Boolean) (Player2Turn :type Boolean))
  ;[1 1 1] Handle Change Turns
  (`self.AskLevelToChangeTurns` Player1Turn Player2Turn))

(event `HandleShipDestroyed`
  (params (ShipSize :type Integer))
  (bind _gamestate (`self.GameState`))
  ;[1 1 1] Notify GameState of Ship Sunk
  (set `/Game/Game/Blueprints/BattleShipGameState.SizeOfShipSunk` ShipSize _gamestate)
  (set `/Game/Game/Blueprints/BattleShipGameState.ShipSunk` true _gamestate))

(event `HandleNotificationOfShipDestroyed`
  (params (ShipSize :type Integer))
  (bind _gamestate (`self.GameState`))
  ;[1 1 1] Show Attacking Player that Opponent's Ship was Sunk
  (`self.IsPlayer#`
    (:`1 (Host)`
      (if (`/Game/Game/Blueprints/BattleShipGameState.Player1Turn` _gamestate)
        (`self.AskLevelToShowOpponentShipSunk` ShipSize :!label _label_6)))
    (:`2 (Client)`
      (if (`/Game/Game/Blueprints/BattleShipGameState.Player2Turn` _gamestate)
        (goto _label_6)))))

(fn `ConfirmShipPlacement`
  ;[1 1 1] Check for correct ship placement
  (`self.AskLevelToConfirmShipPlacement`))

(fn `DisplayConfirmShipPlacement`
  ;[1 1 1] Adds the overlay to confirm ship plaement on ships are placed
  (if (`self.IsLocalPlayerController`)
    (bind _returnvalue (`|CreateWidget` "/Game/Game/UserInterface/ConfirmShipPlacement.ConfirmShipPlacement_C" self))
    (bind _output_get (set `self.ConfirmShipPlacementWidget` _returnvalue))
    (if (`KismetSystemLibrary.IsValid` _output_get)
      (`UserWidget.AddToViewport` _output_get 0)
      (add `/Game/Game/UserInterface/ConfirmShipPlacement.PlacementConfirmed` _output_get (`|CreateDelegate` :!event `ConfirmShipPlacement`)))))

(fn `DisplayConnectingToGameHost`
  ;[1 1 1] Adds the overlay of connecting to host screen
  (if (`self.IsLocalPlayerController`)
    (bind _returnvalue (`|CreateWidget` "/Game/Game/UserInterface/ConnectingToGameHost.ConnectingToGameHost_C" self))
    (bind _output_get (set `self.ConnectingToGameHostWidget` _returnvalue))
    (if (`KismetSystemLibrary.IsValid` _output_get)
      (`UserWidget.AddToViewport` _output_get 1))))

(fn `DisplayDifficultyLevel`
  ;[1 1 1] Displays overlay of Difficulty Level on Screen and calls SetupSinglePlayerMode
  (if (`self.IsLocalPlayerController`)
    (bind _returnvalue (`|CreateWidget` "/Game/Game/UserInterface/DifficultyLevelSelection.DifficultyLevelSelection_C" self))
    (bind _output_get (set `self.DifficultyLevel` _returnvalue))
    (if (`KismetSystemLibrary.IsValid` _output_get)
      (`UserWidget.AddToViewport` _output_get 2)
      (add `/Game/Game/UserInterface/DifficultyLevelSelection.DifficultySelected` _output_get (`|CreateDelegate` :!event `SetupSinglePlayerMode`)))))

(fn `DisplayHostOrJoin`
  ;[1 1 1] Adds the screen overlay to either host or join a game
  (if (`self.IsLocalPlayerController`)
    (bind _returnvalue (`|CreateWidget` "/Game/Game/UserInterface/HostOrJoin.HostOrJoin_C" self))
    (bind _output_get (set `self.HostOrJoinWidget` _returnvalue))
    (if (`KismetSystemLibrary.IsValid` _output_get)
      (`UserWidget.AddToViewport` _output_get 0)
      (add `/Game/Game/UserInterface/HostOrJoin.HostModeSelected` _output_get (`|CreateDelegate` :!event `DisplayShipCountSelect`))
      (add `/Game/Game/UserInterface/HostOrJoin.JoinModeSelected` _output_get (`|CreateDelegate` :!event `SetupClientMode`)))))

(fn `DisplayInvalidShipPlacement`
  ;[1 1 1] Adds the overlay for invalid ship placement
  (if (`self.IsLocalPlayerController`)
    (bind _returnvalue (`|CreateWidget` "/Game/Game/UserInterface/InvalidShipPlacement.InvalidShipPlacement_C" self))
    (bind _output_get (set `self.InvalidShipPlacementWidget` _returnvalue))
    (if (`KismetSystemLibrary.IsValid` _output_get)
      (`UserWidget.AddToViewport` _output_get 0)
      (add `/Game/Game/UserInterface/InvalidShipPlacement.InvalidPlacementAcknowledged` _output_get (`|CreateDelegate` :!event `DisplayConfirmShipPlacement`)))))

(fn `DisplayLose`
  ;[1 1 1] Changes the screen to loser screen
  (if (`self.IsLocalPlayerController`)
    (bind _returnvalue (`|CreateWidget` "/Game/Game/UserInterface/Loser.Loser_C" self))
    (bind _output_get (set `self.LoserWidget` _returnvalue))
    (if (`KismetSystemLibrary.IsValid` _output_get)
      (`UserWidget.AddToViewport` _output_get 3))))

(fn `DisplayShipCountSelect`
  ;[1 1 1] Adds the screen overlay to slect number of ships
  (if (`self.IsLocalPlayerController`)
    (bind _returnvalue (`|CreateWidget` "/Game/Game/UserInterface/ShipQuantitySelection.ShipQuantitySelection_C" self))
    (bind _output_get (set `self.ShipCountSelectWidget` _returnvalue))
    (if (`KismetSystemLibrary.IsValid` _output_get)
      (`UserWidget.AddToViewport` _output_get 0)
      (add `/Game/Game/UserInterface/ShipQuantitySelection.ShipCountSelected` _output_get (`|CreateDelegate` :!event `DisplaySinglePlayer`)))))

(fn `DisplaySinglePlayer`
  ;[1 1 1] Displays Single Player / Host Mode overlay on screen and call difficulty level or SetupHostMode
  (if (`self.IsLocalPlayerController`)
    (bind _returnvalue (`|CreateWidget` "/Game/Game/UserInterface/SinglePlayerSelection.SinglePlayerSelection_C" self))
    (bind _output_get (set `self.SinglePlayerWidget` _returnvalue))
    (if (`KismetSystemLibrary.IsValid` _output_get)
      (`UserWidget.AddToViewport` _output_get 0)
      (add `/Game/Game/UserInterface/SinglePlayerSelection.SinglePlayerModeSelected` _output_get (`|CreateDelegate` :!event `DisplayDifficultyLevel`))
      (add `/Game/Game/UserInterface/SinglePlayerSelection.HostModeSelected` _output_get (`|CreateDelegate` :!event `SetupHostMode`)))))

(fn `DisplayWaitingForPlayerToConnect`
  ;[1 1 1] Takes a given players screen and adds the overlay of waiting to connect
  (if (`self.IsLocalPlayerController`)
    (bind _returnvalue (`|CreateWidget` "/Game/Game/UserInterface/WaitingForPlayerToConnect.WaitingForPlayerToConnect_C" self))
    (bind _output_get (set `self.WaitingForPlayerToConnectWidget` _returnvalue))
    (if (`KismetSystemLibrary.IsValid` _output_get)
      (`UserWidget.AddToViewport` _output_get 2))))

(fn `DisplayWaitingForPlayerToPlaceShips`
  ;[1 1 1] Adds an overlay when opponent is not done placing ships
  (if (`self.IsLocalPlayerController`)
    (bind _returnvalue (`|CreateWidget` "/Game/Game/UserInterface/WaitingForPlayerToPlaceShips.WaitingForPlayerToPlaceShips_C" self))
    (bind _output_get (set `self.WaitingForPlayerToPlaceShipsWidget` _returnvalue))
    (if (`KismetSystemLibrary.IsValid` _output_get)
      (`UserWidget.AddToViewport` _output_get 2))))

(fn `DisplayWin`
  ;[1 1 1] Changes the screen to display a win
  (if (`self.IsLocalPlayerController`)
    (bind _returnvalue (`|CreateWidget` "/Game/Game/UserInterface/Winner.Winner_C" self))
    (bind _output_get (set `self.WinnerWidget` _returnvalue))
    (if (`KismetSystemLibrary.IsValid` _output_get)
      (`UserWidget.AddToViewport` _output_get 3))))

(fn `RemoveConfirmShipPlacement`
  (params (Remove :type Boolean))
  (bind _confirmshipplacementwidget (`self.ConfirmShipPlacementWidget`))
  ;[1 1 1] Deletes the overlay of confirming ship placement
  (if Remove
    (if (`KismetSystemLibrary.IsValid` _confirmshipplacementwidget)
      (`Widget.RemoveFromParent` _confirmshipplacementwidget))))

(fn `RemoveConnectingToGameHost`
  (params (Remove :type Boolean))
  (bind _connectingtogamehostwidget (`self.ConnectingToGameHostWidget`))
  ;[1 1 1] Deletes the overlay of conecting to game screen
  (if Remove
    (if (`KismetSystemLibrary.IsValid` _connectingtogamehostwidget)
      (`Widget.RemoveFromParent` _connectingtogamehostwidget))))

(fn `RemoveDifficultyLevel`
  (params (Remove :type Boolean))
  (bind _difficultylevel (`self.DifficultyLevel`))
  ;[1 1 1] Deletes the difficulty level overlay
  (if Remove
    (if (`KismetSystemLibrary.IsValid` _difficultylevel)
      (`Widget.RemoveFromParent` _difficultylevel))))

(fn `RemoveHostOrJoin`
  (params (Remove :type Boolean))
  (bind _hostorjoinwidget (`self.HostOrJoinWidget`))
  ;[1 1 1] Deletes the overlay of the host or join screen
  (if Remove
    (if (`KismetSystemLibrary.IsValid` _hostorjoinwidget)
      (`Widget.RemoveFromParent` _hostorjoinwidget))))

(fn `RemoveInvalidShipPlacement`
  (params (Remove :type Boolean))
  (bind _invalidshipplacementwidget (`self.InvalidShipPlacementWidget`))
  ;[1 1 1] Deletes the overlay for invalid ship placement
  (if Remove
    (if (`KismetSystemLibrary.IsValid` _invalidshipplacementwidget)
      (`Widget.RemoveFromParent` _invalidshipplacementwidget))))

(fn `RemoveShipCountSelect`
  (bind _shipcountselectwidget (`self.ShipCountSelectWidget`))
  ;[1 1 1] Deletes the screen overlay to select number of ships
  (if true
    (if (`KismetSystemLibrary.IsValid` _shipcountselectwidget)
      (`Widget.RemoveFromParent` _shipcountselectwidget))))

(fn `RemoveSinglePlayer`
  (params (Remove :type Boolean))
  (bind _singleplayerwidget (`self.SinglePlayerWidget`))
  ;[1 1 1] Deletes the singleplayer overlay
  (if Remove
    (if (`KismetSystemLibrary.IsValid` _singleplayerwidget)
      (`Widget.RemoveFromParent` _singleplayerwidget))))

(fn `RemoveWaitingForPlayerToConnect`
  (params (Remove :type Boolean))
  (bind _waitingforplayertoconnectwidget (`self.WaitingForPlayerToConnectWidget`))
  ;[1 1 1] Deletes the overlay of Waiting for player to connect screen
  (if Remove
    (if (`KismetSystemLibrary.IsValid` _waitingforplayertoconnectwidget)
      (`Widget.RemoveFromParent` _waitingforplayertoconnectwidget))))

(fn `RemoveWaitingForPlayerToPlaceShips`
  (params (Remove :type Boolean))
  (bind _waitingforplayertoplaceshipswidget (`self.WaitingForPlayerToPlaceShipsWidget`))
  ;[1 1 1] Deletes the overlay of waiting for player to connect ships
  (if Remove
    (if (`KismetSystemLibrary.IsValid` _waitingforplayertoplaceshipswidget)
      (`Widget.RemoveFromParent` _waitingforplayertoplaceshipswidget))))

(fn `SetupPlayer1Bindings`
  (bind _gamestate (`self.GameState`))
  ;[1 1 1] Binds Player 1 To Game
  (add `/Game/Game/Blueprints/BattleShipGameState.NotifyPlayer2Connected` _gamestate (`|CreateDelegate` :!event `RemoveWaitingForPlayerToConnect`))
  (add `/Game/Game/Blueprints/BattleShipGameState.NotifyPlayerWinLose` _gamestate (`|CreateDelegate` :!event `DisplayWinLose`)))

(fn `SetupPlayer1BindingsPart2`
  (bind _gamestate (`self.GameState`))
  ;[1 1 1] Removes Player1 from waiting Screen, Adds Player1 to a team and Turn on ShipDestroyed Notifications
  (add `/Game/Game/Blueprints/BattleShipGameState.NotifyPlayer2Ready` _gamestate (`|CreateDelegate` :!event `RemoveWaitingForPlayerToPlaceShips`))
  (add `/Game/Game/Blueprints/BattleShipGameState.NotifyChangeTurns` _gamestate (`|CreateDelegate` :!event `HandleChangeTurns`))
  (add `/Game/Game/Blueprints/BattleShipGameState.NotifyShipSunk` _gamestate (`|CreateDelegate` :!event `HandleNotificationOfShipDestroyed`)))

(fn `SetupPlayer2Bindings`
  (bind _gamestate (`self.GameState`))
  ;[1 1 1] Binds Player Two to Game
  (add `/Game/Game/Blueprints/BattleShipGameState.NotifyPlayer2Connected` _gamestate (`|CreateDelegate` :!event `RemoveConnectingToGameHost`))
  (add `/Game/Game/Blueprints/BattleShipGameState.NotifyPlayerWinLose` _gamestate (`|CreateDelegate` :!event `DisplayWinLose`)))

(fn `SetupPlayer2BindingsPart2`
  (bind _gamestate (`self.GameState`))
  ;[1 1 1] Removes Player2 from waiting Screen, Adds Player2 to a team and Turn on ShipDestroyed Notifications
  (add `/Game/Game/Blueprints/BattleShipGameState.NotifyPlayer1Ready` _gamestate (`|CreateDelegate` :!event `RemoveWaitingForPlayerToPlaceShips`))
  (add `/Game/Game/Blueprints/BattleShipGameState.NotifyChangeTurns` _gamestate (`|CreateDelegate` :!event `HandleChangeTurns`))
  (add `/Game/Game/Blueprints/BattleShipGameState.NotifyShipSunk` _gamestate (`|CreateDelegate` :!event `HandleNotificationOfShipDestroyed`)))

(fn `UserConstructionScript`)