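; Game board actor that animates a pop-up and opening motion, staged for the Opening_Animation level.
; On BeginPlay in that level, it presets the Scene component to a starting height and roll.
; The Animate event plays a timeline driving Scene's relative Z, then on finish chains a second timeline driving its roll to open the board.
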(event `self.ReceiveBeginPlay`
  (bind _scene (`self.Scene`))
  (bind (_relativerotation_roll _relativerotation_pitch _relativerotation_yaw) (`KismetMathLibrary.BreakRotator` (`SceneComponent.RelativeRotation` _scene)))
  (bind (_relativelocation_x _relativelocation_y) (`KismetMathLibrary.BreakVector` (`SceneComponent.RelativeLocation` _scene)))
  (bind _returnvalue (`GameplayStatics.GetCurrentLevelName` true))
  (if (`KismetStringLibrary.EqualEqual_StrStr` _returnvalue "Opening_Animation")
    (`SceneComponent.K2_SetRelativeLocation` _scene (`KismetMathLibrary.MakeVector` _relativelocation_x _relativelocation_y -35.0) false false)
    (`SceneComponent.K2_SetRelativeRotation` _scene (`KismetMathLibrary.MakeRotator` 120.0 _relativerotation_pitch _relativerotation_yaw) false false)))

(event `Animate`
  (bind _scene (`self.Scene`))
  (bind _scene_2 (`self.Scene`))
  (bind (_relativelocation_x _relativelocation_y) (`KismetMathLibrary.BreakVector` (`SceneComponent.RelativeLocation` _scene)))
  (bind (_relativerotation_roll _relativerotation_pitch _relativerotation_yaw) (`KismetMathLibrary.BreakRotator` (`SceneComponent.RelativeRotation` _scene_2)))
  (bind (_direction _height) (`Timeline|PopGameBoardTimeline` :!via `PlayFromStart`)
    (:`Update`
      (`SceneComponent.K2_SetRelativeLocation` _scene (`KismetMathLibrary.MakeVector` _relativelocation_x _relativelocation_y _height) false false))
    (:`Finished`
      (bind (_direction_2 _angle) (`Timeline|OpenGameBoardTimeline` :!via `PlayFromStart`)
        (:`Update`
          (`SceneComponent.K2_SetRelativeRotation` _scene_2 (`KismetMathLibrary.MakeRotator` _angle _relativerotation_pitch _relativerotation_yaw) false false))))))

(fn `UserConstructionScript`)